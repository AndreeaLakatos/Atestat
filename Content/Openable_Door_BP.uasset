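; Swinging door for BuildingEscape, driven by its OpenDoor component's open and close events.
; The DoorSwing timeline plays or reverses, adding a yaw offset to the stored initial rotation, with a DoOnce-gated lock sound when it finishes closing.
; On BeginPlay it stores its rotation and registers in the game mode's Usa1 array.
; A separate Open event snaps it to a fixed rotation, makes that the new base and plays the lock sound.
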(event OnClose(OpenDoor)
  (bind (_direction _open_angle) (Timeline|Door%20Swing Reverse)
    (:Update
      (Transformation|SetActorRotation (Math|Rotator|CombineRotators (Math|Rotator|MakeRotator 0.0 0.0 _open_angle) (Variables|Default|GetInitialRotation))))
    (:Finished
      (if (Utilities|Enum|Equal(Enum) _direction "Backward")
        (Utilities|FlowControl|DoOnce false :!label _label
          (:Completed
            (Audio|PlaySoundatLocation "/Game/Audio/door-lock.door-lock" (Transformation|GetActorLocation) "0, 0, 0" 1.0 1.0 0.0 0 0 0)))
        (else
          (goto _label Reset))))))

(event OnOpen(OpenDoor)
  (Utilities|FlowControl|Sequence
    (:then_1
      (bind (_direction _open_angle) (Timeline|Door%20Swing Play)
        (:Update
          (Transformation|SetActorRotation (Math|Rotator|CombineRotators (Math|Rotator|MakeRotator 0.0 0.0 _open_angle) (Variables|Default|GetInitialRotation))))
        (:Finished
          (if (Utilities|Enum|Equal(Enum) _direction "Backward")
            (Utilities|FlowControl|DoOnce false :!label _label
              (:Completed
                (Audio|PlaySoundatLocation "/Game/Audio/door-lock.door-lock" (Transformation|GetActorLocation) "0, 0, 0" 1.0 1.0 0.0 0 0 0)))
            (else
              (goto _label Reset))))))))

(event Custom|Open
  (bind _output_get (Variables|Default|SetInitialRotation "0,-80.000000, 0"))
  (Transformation|SetActorRotation _output_get)
  (Audio|PlaySoundatLocation "/Game/Audio/door-lock.door-lock" (Transformation|GetActorLocation) "0, 0, 0" 1.0 1.0 0.0 0 0 0))

(event EventBeginPlay
  (Variables|Default|SetInitialRotation (Transformation|GetActorRotation))
  (bind _asbuilding_escape_game_mode_bp (Utilities|Casting|CastToBuildingEscapeGameMode_BP (Game|GetGameMode)))
  (Utilities|Array|Add (Variables|/Game/BuildingEscapeGameMode_BP.BuildingEscapeGameMode_BP_C|GetUsa%201 _asbuilding_escape_game_mode_bp) self))

(fn ConstructionScript)